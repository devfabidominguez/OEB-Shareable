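; Behavior tree decorator that gates execution on a waypoint index counter in the OEB_AIController's blackboard, acting as a countdown loop condition.
; Each condition check reads WaypointCurrentIndex and passes if it is above zero.
; The check also has a side effect: it writes the index back decremented by one, even when the condition fails.
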(fn PerformConditionCheck
  (params (OwnerActor :type Actor%20Object%20Reference))
  (bind _asoeb_aicontroller (Utilities|Casting|CastToOEB_AIController OwnerActor))
  (bind _output_get (LocalVariables|SetShouldExecute (> (Class|BlackboardComponent|GetValueasInt (Variables|/Game/Blueprints/AI/OEB_AIController.OEB_AIController_C|GetBlackboardComponent _asoeb_aicontroller) (LocalVariables|GetWaypointCurrentIndex)) 0)))
  (Class|BlackboardComponent|SetValueasInt (Variables|/Game/Blueprints/AI/OEB_AIController.OEB_AIController_C|GetBlackboardComponent _asoeb_aicontroller) (LocalVariables|GetWaypointCurrentIndex) (- (Class|BlackboardComponent|GetValueasInt (Variables|/Game/Blueprints/AI/OEB_AIController.OEB_AIController_C|GetBlackboardComponent _asoeb_aicontroller) (LocalVariables|GetWaypointCurrentIndex)) 1))
  (return _output_get))