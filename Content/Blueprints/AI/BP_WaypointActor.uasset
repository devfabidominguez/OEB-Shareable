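; BP_WaypointActor is an AI waypoint marker that can impose a cooldown on AI characters within its sphere.
; On BeginPlay it hides itself unless SeenInGame is set.
; When CooldownTime is positive, it calls TryApplyWaypointCooldown on each BP_AICharacter already overlapping the sphere at BeginPlay and on any that enters later, passing itself and the duration.
; The cooldown logic itself lives in the AI character.
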(event OnComponentBeginOverlap(Sphere)
  (params (OverlappedComponent :type Primitive%20Component%20Object%20Reference) (OtherActor :type Actor%20Object%20Reference) (OtherComp :type Primitive%20Component%20Object%20Reference) (OtherBodyIndex :type Integer) (bFromSweep :type Boolean) (SweepResult :type Hit%20Result%20Structure%20%28by%20ref%29))
  (if (> (Variables|Default|GetCooldownTime) 0.0)
    (bind _asbp_aicharacter (Utilities|Casting|CastToBP_AICharacter OtherActor))
    (Default|TryApplyWaypointCooldown _asbp_aicharacter (Variables|Default|GetCooldownTime) self)))

(event EventBeginPlay
  (Rendering|SetActorHiddenInGame (not (Variables|Default|GetSeenInGame)))
  (if (> (Variables|Default|GetCooldownTime) 0.0)
    (for _array_element (Collision|GetOverlappingActors (Variables|Default|GetSphere) "/Game/ThirdPersonCPP/Blueprints/BP_AICharacter.BP_AICharacter_C" :!class /Script/Engine.PrimitiveComponent)
      (bind _asbp_aicharacter (Utilities|Casting|CastToBP_AICharacter _array_element))
      (Default|TryApplyWaypointCooldown _asbp_aicharacter (Variables|Default|GetCooldownTime) self))))

(event Collision|EventActorBeginOverlap
  (params (OtherActor :type Actor%20Object%20Reference)))

(event EventTick
  (params (DeltaSeconds :type Float%20%28single-precision%29)))

(fn ConstructionScript)