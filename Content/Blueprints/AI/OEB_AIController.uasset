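; AI controller that runs the OEB base behavior tree and blackboard for its pawn.
; On BeginPlay it sets up the blackboard, stores the controlled pawn as self actor and starts the tree.
; AI perception writes any visible BP_PenaltyBall it senses as the target ball.
; Helper functions write the waypoint, waypoint index and cooldown keys, and check whether an actor is the current waypoint.
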(event OnTargetPerceptionUpdated(AIPerception)
  (params (Actor :type Actor%20Object%20Reference) (Stimulus :type AI%20Stimulus%20Structure))
  (bind _asbp_penalty_ball (Utilities|Casting|CastToBP_PenaltyBall Actor))
  (if (not (Variables|/Script/Engine.Actor|GetbHidden _asbp_penalty_ball))
    (AI|Components|Blackboard|SetValueasObject (Variables|Default|GetBlackboard) (Variables|Default|GetName_TargetBall) _asbp_penalty_ball)))

(event EventBeginPlay
  (bind (_blackboardcomponent _returnvalue) (Class|AIController|UseBlackboard "/Game/Blueprints/AI/OEB_AIBaseBlackboard.OEB_AIBaseBlackboard"))
  (if _returnvalue
    (bind _output_get (Variables|Default|SetBlackboardComponent _blackboardcomponent))
    (AI|Components|Blackboard|SetValueasObject _output_get (Variables|Default|GetName_SelfActor) (Pawn|GetControlledPawn))
    (Development|PrintString "Set Blackboard")
    (bind _returnvalue_2 (AI|RunBehaviorTree "/Game/Blueprints/AI/OEB_AIBaseTree.OEB_AIBaseTree"))
    (if _returnvalue_2
      (Development|PrintString "Run Behavior Tree"))))

(event EventTick
  (params (DeltaSeconds :type Float%20%28single-precision%29)))

(fn ConstructionScript)

(fn UpdateWaypoint
  (params (NewWaypoint :type Actor%20Object%20Reference%20%28by%20ref%29))
  (AI|Components|Blackboard|SetValueasObject (Variables|Default|GetBlackboardComponent) (Variables|Default|GetName_Waypoint) NewWaypoint))

(fn IsActorTargetWaypoint
  (params (Actor :type Actor%20Object%20Reference))
  (return (== Actor (AI|Components|Blackboard|GetValueasObject (Variables|Default|GetBlackboardComponent) (Variables|Default|GetName_Waypoint)))))

(fn UpdateCooldown
  (params (CooldownTime :type Float%20%28single-precision%29))
  (AI|Components|Blackboard|SetValueasFloat (Variables|Default|GetBlackboardComponent) (Variables|Default|GetName_Cooldown) CooldownTime))

(fn UpdateCurrentIndex
  (params (NewWaypointIndex :type Integer))
  (Class|BlackboardComponent|SetValueasInt (Variables|Default|GetBlackboardComponent) (Variables|Default|GetName_WaypointIndex) NewWaypointIndex))