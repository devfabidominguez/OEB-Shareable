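; Component for a BP_CineCamera owner that makes the camera follow a skeletal mesh bone while facing its look-at tracking target.
; On Tick, when custom tick is enabled, it rotates the owner toward that actor and reads the BoneFollow socket location.
; It adds hardcoded camera-forward, up and Z offsets, then lerps the owner there by delta time.
; The configurable offset and InterpSpeed helper paths are not used by Tick.
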(event Custom|CallSetupTransform)

(event EventBeginPlay
  (Transformation|SetActorTransform (Components|GetOwner) (Variables|Default|GetSetupTransform))
  (Variables|Default|SetCameraComponent (Actor|GetComponentbyClass (Components|GetOwner) "/Script/Engine.CameraComponent"))
  (CallFunction|UpdateValidTargetLocation (Variables|Default|GetSkeletal_Parent)))

(event EventTick
  (params (DeltaSeconds :type Float%20%28single-precision%29))
  (Variables|Default|SetOffsetChanged (not (Math|Vector|Equal(Vector) (Variables|Default|GetOffSetLocation) (Variables|Default|GetLastTargetLocation) 0.0001)))
  (if (Variables|Default|GetCustomTickEnabled)
    (Utilities|GetValidSkeletal
      (:Valid
        (CallFunction|UpdateRotationtoLookatObject)
        (CallFunction|UpdateValidTargetLocation (Variables|Default|GetSkeletal_Parent))
        (CallFunction|OffsetTargetLocation)
        (Transformation|SetActorLocation (Components|GetOwner) (Math|Vector|Lerp(Vector) (Transformation|GetActorLocation (Components|GetOwner)) (Variables|Default|GetTargetLocation) (* 10 (Utilities|Time|GetWorldDeltaSeconds))) false false)))))

(fn UpdateValidTargetLocation
  (params (NewParam :type Skeletal%20Mesh%20Actor%20Object%20Reference))
  (bind _newparam (Utilities|GetValidSkeletal)
    (:Valid
      (Variables|Default|SetTargetLocation (Transformation|GetSocketLocation (Variables|/Script/Engine.SkeletalMeshActor|GetSkeletalMeshComponent _newparam) (Variables|Default|GetBoneFollow))))))

(fn LerptoTargetLocation
  (params (Delta :type Float%20%28single-precision%29))
  (bind _cameracomponent (Variables|Default|GetCameraComponent))
  (bind _interpolated (CallFunction|VInterpCasero (Variables|/Script/Engine.SceneComponent|GetRelativeLocation _cameracomponent) (Variables|Default|GetTargetLocation) Delta (Variables|Default|GetInterpSpeed)))
  (Transformation|SetRelativeLocation _cameracomponent _interpolated false false))

(fn VInterpCasero
  (params (Current :type Vector) (Target :type Vector) (DeltaTime :type Float%20%28single-precision%29) (InterpSpeed :type Float%20%28single-precision%29))
  (bind _returnvalue (- Target Current))
  (if (<= InterpSpeed 0.0)
    _
    (else
      (LocalVariables|SetDist _returnvalue)
      (if (< (Math|Vector|VectorLengthSquared _returnvalue) 0.0001)
        _
        (else
          (return (+ (* (LocalVariables|GetDist) (* DeltaTime InterpSpeed)) Current) true)))))
  ;[1 1 1] Return Target As Is
  (return Target false))

(fn OffsetTargetLocation
  (if (Variables|Default|GetFollowBoneForward)
    _
    (else
      _))
  (CallFunction|UpdateTargetLocationForward))

(fn UpdateDefaultTargetLocation
  (bind _cameracomponent (Variables|Default|GetCameraComponent))
  (Utilities|IsValid _cameracomponent
    (:Is%20Valid
      (Variables|Default|SetTargetLocation (+ (Variables|Default|GetTargetLocation) (* (Math|Vector|GetForwardVector _cameracomponent) (Variables|Default|GetOffSetLocation)) (Variables|Default|GetOffsetFlat))))))

(fn UpdateTargetLocationForward
  (bind _cameracomponent (Variables|Default|GetCameraComponent))
  (Utilities|IsValid _cameracomponent
    (:Is%20Valid
      (bind _output_get (Variables|Default|SetTargetLocation (+ (Variables|Default|GetTargetLocation) (* (Math|Vector|GetForwardVector _cameracomponent) 45) (* (Math|Vector|GetUpVector _cameracomponent) 20))))
      (Variables|Default|SetTargetLocation (Math|Vector|MakeVector (.x _output_get) (.y _output_get) (+ (.z _output_get) 25.0))))))

(fn UpdateRotationtoLookatObject
  (bind _returnvalue (Components|GetOwner))
  (bind (_lookatobject _haschanged) (CallFunction|GetLookatObject))
  (Utilities|IsValid _lookatobject
    (:Is%20Valid
      (if _haschanged
        _
        (else
          _))
      (Variables|Default|SetTargetRotation (Transformation|GetActorRotation _lookatobject))
      (Transformation|SetActorRotation _returnvalue (Math|Rotator|FindLookatRotation (Transformation|GetActorLocation _returnvalue) (Transformation|GetActorLocation _lookatobject))))))

(fn GetLookatObject
  (bind _asbp_cine_camera (Utilities|Casting|CastToBP_CineCamera (Components|GetOwner)))
  (bind _returnvalue (Utilities|LoadAssetBlocking (.actortotrack (Variables|/Script/CinematicCamera.CineCameraActor|GetLookatTrackingSettings _asbp_cine_camera))))
  (bind _asactor (Utilities|Casting|CastToActor _returnvalue))
  (bind _output_get (Variables|Default|SetLookAtSettings _asactor))
  (return _output_get false))