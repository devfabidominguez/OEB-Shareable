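; BP_PenaltyBall is the ball actor for penalty shots, launched via ProjectileMovement with a configurable LaunchVelocity.
; It starts with simulation off, can attach to a character's RightHand socket and detach, and exposes events to move, reset, start, shoot and stop it.
; Tick spins the separate Visual component according to velocity direction while RotationSpeed is positive.
; An editor helper draws the predicted projectile path.
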(event Custom|ResetPosition
  (Transformation|SetWorldLocation (Variables|Default|GetMesh) (Variables|Default|GetStartPosition) false true))

(event Custom|Start%20Simulation
  (Transformation|SetWorldRotation (Variables|Default|GetMesh) "0, 0, 0" false false)
  (Variables|/Script/Engine.ProjectileMovementComponent|SetbSimulationEnabled (Variables|Default|GetProjectileMovement) true))

(event Custom|Editor_ShowProjectilePrediction
  (bind _mesh (Variables|Default|GetMesh))
  (Class|GameplayStatics|BlueprintPredictProjectilePathAdvanced (Utilities|Struct|MakePredictProjectilePathParams (Transformation|GetWorldLocation _mesh) (Variables|Default|GetLaunchVelocity) false (.SphereRadius (Collision|GetComponentBounds _mesh)) 1.0 true "ECC_WorldStatic" "ObjectTypeQuery1" 0 2e+01 0.0 "ForDuration" 1.0 false)))

(event Custom|Move
  (params (Direction :type Vector))
  (bind _mesh (Variables|Default|GetMesh))
  (bind _returnvalue (Transformation|GetWorldLocation _mesh))
  (bind _returnvalue_2 (+ _returnvalue Direction))
  (Transformation|SetWorldLocation _mesh _returnvalue_2 false true)
  (Variables|Default|SetStartPosition _returnvalue_2))

(event Custom|SetupPenaltyPosition
  (Transformation|AttachActorToActor (Variables|Default|GetCharacterSkeleton) "RightHand" "KeepRelative" "KeepRelative" "KeepRelative" false)
  (Transformation|SetActorRelativeLocation (Variables|Default|GetSetupPosition) false true))

(event Custom|ShootPenalty
  (Game|Components|ProjectileMovement|SetVelocityinLocalSpace (Variables|Default|GetProjectileMovement) (Variables|Default|GetLaunchVelocity)))

(event Custom|StopSimulation
  (bind _projectilemovement (Variables|Default|GetProjectileMovement))
  (Components|Movement|StopMovementImmediately _projectilemovement)
  (Variables|/Script/Engine.ProjectileMovementComponent|SetbSimulationEnabled _projectilemovement false))

(event Custom|Test
  (CallFunction|StartSimulation)
  (CallFunction|ShootPenalty))

(event Custom|StopRotation
  (Variables|Default|SetRotationSpeed -1.0))

(event Custom|AffectVisual
  (params (Hidden :type Boolean))
  (Development|SetHiddeninGame (Variables|Default|GetVisual) Hidden false)
  (Collision|SetCollisionEnabled (Variables|Default|GetMesh) (select Hidden "NoCollision" "QueryAndPhysics")))

(event EventBeginPlay
  (CallFunction|InitSequence))

(event Collision|EventActorBeginOverlap
  (params (OtherActor :type Actor%20Object%20Reference)))

(event EventTick
  (params (DeltaSeconds :type Float%20%28single-precision%29))
  (bind _returnvalue (Transformation|GetActorLocation))
  (bind _visual (Variables|Default|GetVisual))
  (bind _returnvalue_2 (Transformation|GetWorldRotation _visual))
  (if (> (Variables|Default|GetRotationSpeed) 0.0)
    (Transformation|SetWorldRotation (Variables|Default|GetVisual) (Math|Interpolation|RInterpTo _returnvalue_2 (Math|Rotator|CombineRotators _returnvalue_2 (Math|Rotator|FindLookatRotation _returnvalue (+ _returnvalue (Variables|/Script/Engine.MovementComponent|GetVelocity (Variables|Default|GetProjectileMovement))))) DeltaSeconds (Variables|Default|GetRotationSpeed)) false false)))

(event EventDetachBall
  (Transformation|DetachFromActor "KeepWorld" "KeepWorld" "KeepWorld"))

(fn ConstructionScript)

(fn InitSequence
  (bind _mesh (Variables|Default|GetMesh))
  (Variables|Default|SetStartPosition (Transformation|GetWorldLocation _mesh))
  (Variables|Default|SetStartRotation (Transformation|GetWorldRotation _mesh))
  (Variables|/Script/Engine.ProjectileMovementComponent|SetbSimulationEnabled (Variables|Default|GetProjectileMovement) false)
  (Rendering|SetActorHiddenInGame (Variables|Default|GetStartHidden))
  (Collision|SetActorEnableCollision (Variables|Default|GetStartCollisioning)))