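; BP_ERController_Base is a base ER controller that manages an on-screen meter for ER progress.
; On BeginPlay it creates a Widget_Measure for player 0 and adds it to the viewport.
; Each Tick it polls ERActorComponent, when valid, and pushes its progress into the widget.
; Two helper functions hide the widget or show it as hit-test invisible.
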(event EventBeginPlay
  (bind _returnvalue (UserInterface|CreateWidget "/Game/UI/Widget_Measure.Widget_Measure_C" (Game|GetPlayerController 0)))
  (bind _output_get (Variables|Default|SetERWidget _returnvalue))
  (UserInterface|Viewport|AddtoViewport _output_get 0))

(event EventTick
  (params (DeltaSeconds :type Float%20%28single-precision%29))
  (Utilities|IsValid (Variables|Default|GetERActorComponent)
    (:Is%20Valid
      (bind _aswidget_measure (Utilities|Casting|CastToWidget_Measure (Variables|Default|GetERWidget))
        (:then
          (Default|SetERProgress _aswidget_measure (Class|ERActorComponent|GetERProgress (Variables|Default|GetERActorComponent))))
        (:CastFailed
          (Development|PrintString "Hello"))))))

(fn ConstructionScript)

(fn HideERWidget
  (Widget|SetVisibility (Variables|Default|GetERWidget) "Hidden"))

(fn ShowERWidget
  (Widget|SetVisibility (Variables|Default|GetERWidget) "HitTestInvisible"))