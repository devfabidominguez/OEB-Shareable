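; Game mode for a VR game that, on BeginPlay, disables on-screen messages to avoid Oculus crashes and spawns a BP_ERController_Base.
; ConnectActorToERController gives that controller the passed actor's BP_ERActorComponent_Goal, only while it holds no valid component.
; Spectator-screen code for showing a widget beside the eye view is disconnected, leaving ShowMierda empty and HideSpectatorWidget uncalled within this graph.
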(event Custom|ShowMierda
  (params (NewParam :type Boolean)))

(event EventBeginPlay
  (CallFunction|ExecuteConsoleCommands)
  (CallFunction|SpawnERController))

(event EventTick
  (params (DeltaSeconds :type Float%20%28single-precision%29)))

(fn ConstructionScript)

(fn HideSpectatorWidget
  (Class|WidgetComponent|SetTickwhenOffscreen (Variables|Default|GetWidget) false)
  (Class|HeadMountedDisplayFunctionLibrary|SetSpectatorScreenMode "SingleEyeCroppedToFill"))

(fn SpawnERController
  (bind _returnvalue (Game|SpawnActorfromClass "/Game/Blueprints/ER/BP_ERController_Base.BP_ERController_Base_C" (Math|Transform|MakeTransform "0, 0, 0") "Undefined" self 0))
  (Variables|Default|SetERController _returnvalue))

(fn ExecuteConsoleCommands
  ;[1 1 1] Ocullus can crash for using screen messages
  (Development|ExecuteConsoleCommand "DisableAllScreenMessages" 0))

(fn ConnectActortoERController
  (params (ActorToConnect :type Actor%20Object%20Reference))
  (bind _ercontroller (Variables|Default|GetERController))
  (Utilities|IsValid (Variables|/Game/Blueprints/ER/BP_ERController_Base.BP_ERController_Base_C|GetERActorComponent _ercontroller)
    (:Is%20Not%20Valid
      (Variables|/Game/Blueprints/ER/BP_ERController_Base.BP_ERController_Base_C|SetERActorComponent _ercontroller (Actor|GetComponentbyClass ActorToConnect "/Game/Blueprints/ER/BP_ERActorComponent_Goal.BP_ERActorComponent_Goal_C")))))