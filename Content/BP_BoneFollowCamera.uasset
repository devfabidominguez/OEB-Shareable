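; Camera actor that follows a named bone or socket on a parent skeletal mesh actor.
; BeginPlay snap-attaches it to that bone and disables tick when the parent is valid, so attachment does the following.
; The dormant Tick path moves it to the bone, aims it at the look-at tracking actor and accumulates an offset into TargetLocation.
; The custom VInterp smoothing is disconnected, so that offset never moves the camera.
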(event EventBeginPlay
  ;[1 1 1] Algorithm assumes bone is 0.0.0 relative initially
  (bind _mesh (Utilities|GetvalidSkeletal)
    (:Valid
      (Transformation|AttachActorToActor _mesh (Variables|Default|GetBoneFollow) "SnapToTarget" "SnapToTarget" "SnapToTarget" true)
      (Actor|Tick|SetActorTickEnabled false))))

(event Collision|EventActorBeginOverlap
  (params (OtherActor :type Actor%20Object%20Reference))
  ;[1 1 1] Algorithm assumes bone is 0.0.0 relative initially
)

(event EventTick
  (params (DeltaSeconds :type Float%20%28single-precision%29))
  (Utilities|GetvalidSkeletal
    (:Valid
      (CallFunction|UpdateTargetLocation)
      (CallFunction|OffsetTargetLocation)
      (CallFunction|LerptoTargetLocation DeltaSeconds))))

(fn ConstructionScript)

(fn UpdateTargetLocation
  (bind _returnvalue (Transformation|GetActorLocation))
  (bind _bonefollow (Variables|Default|GetBoneFollow))
  (bind _lookattrackingsettings (Variables|Default|GetLookatTrackingSettings))
  (bind _output (Utilities|ResolveSoftReference (.actortotrack _lookattrackingsettings)))
  (bind _returnvalue_2 (Transformation|GetActorLocation _output))
  (bind _returnvalue_3 (Math|Rotator|FindLookatRotation _returnvalue _returnvalue_2))
  (bind _mesh (Utilities|GetvalidSkeletal)
    (:Valid
      (Transformation|SetActorLocation (Transformation|GetSocketLocation (Variables|/Script/Engine.SkeletalMeshActor|GetSkeletalMeshComponent _mesh) _bonefollow) false false)
      (Variables|Default|SetTargetRotation (Transformation|GetSocketRotation (Variables|/Script/Engine.SkeletalMeshActor|GetSkeletalMeshComponent _mesh) _bonefollow))
      (Transformation|SetActorRotation (Math|Rotator|MakeRotator (.roll _returnvalue_3) (.pitch _returnvalue_3) (.yaw _returnvalue_3))))))

(fn LerptoTargetLocation
  (params (Delta :type Float%20%28single-precision%29)))

(fn OffsetTargetLocation
  (Variables|Default|SetTargetLocation (+ (Variables|Default|GetTargetLocation) (* (Math|Vector|GetForwardVector (Variables|CameraActor|GetCameraComponent)) (Variables|Default|GetOffSetLocation)) (Variables|Default|GetOffsetFlat))))

(fn VInterptoCasero
  (params (Current :type Vector) (Target :type Vector) (DeltaTime :type Float%20%28single-precision%29) (InterpSpeed :type Float%20%28single-precision%29))
  (if (<= InterpSpeed 0.0)
    _
    (else
      (bind _output_get (LocalVariables|SetDist (- Target Current)))
      (if (< (Math|Vector|VectorLengthSquared _output_get) 0.0001)
        _
        (else
          (return (+ (* (LocalVariables|GetDist) (* DeltaTime InterpSpeed)) Current))))))
  ;[1 1 1] Return Target As Is
  (return Target))