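; Penalty ball actor that launches through a ProjectileMovement component, with simulation off until explicitly started.
; Events attach it to a character's RightHand socket, toggle simulation, and fire it with LaunchVelocity in local space.
; It records its starting location for resets, and Move shifts both the mesh and that stored position.
; An Editor_ShowProjectilePrediction event draws the predicted flight path from the current location and launch velocity.
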(event Custom|ResetPosition
  (Transformation|SetWorldLocation (Variables|Default|GetMesh) (Variables|Default|GetStartPosition) false true))

(event Custom|Start%20Simulation
  (Transformation|SetWorldRotation (Variables|Default|GetMesh) "0, 0, 0" false false)
  (Variables|/Script/Engine.ProjectileMovementComponent|SetbSimulationEnabled (Variables|Default|GetProjectileMovement) true))

(event Custom|Editor_ShowProjectilePrediction
  (bind _mesh (Variables|Default|GetMesh))
  (Class|GameplayStatics|BlueprintPredictProjectilePathAdvanced (Utilities|Struct|MakePredictProjectilePathParams (Transformation|GetWorldLocation _mesh) (Variables|Default|GetLaunchVelocity) false (.SphereRadius (Collision|GetComponentBounds _mesh)) 1.0 true "ECC_WorldStatic" "ObjectTypeQuery1" 0 2e+01 0.0 "ForDuration" 1.0 false)))

(event Custom|Move
  (params (Direction :type Vector))
  (bind _mesh (Variables|Default|GetMesh))
  (bind _returnvalue (Transformation|GetWorldLocation _mesh))
  (bind _returnvalue_2 (+ _returnvalue Direction))
  (Transformation|SetWorldLocation _mesh _returnvalue_2 false true)
  (Variables|Default|SetStartPosition _returnvalue_2))

(event Custom|SetupPenaltyPosition
  (Transformation|AttachActorToActor (Variables|Default|GetCharacterSkeleton) "RightHand" "KeepRelative" "KeepRelative" "KeepRelative" false)
  (Transformation|SetActorRelativeLocation (Variables|Default|GetSetupPosition) false true))

(event Custom|ShootPenalty
  (Game|Components|ProjectileMovement|SetVelocityinLocalSpace (Variables|Default|GetProjectileMovement) (Variables|Default|GetLaunchVelocity)))

(event Custom|StopSimulation
  (bind _projectilemovement (Variables|Default|GetProjectileMovement))
  (Components|Movement|StopMovementImmediately _projectilemovement)
  (Variables|/Script/Engine.ProjectileMovementComponent|SetbSimulationEnabled _projectilemovement false))

(event EventBeginPlay
  (bind _mesh (Variables|Default|GetMesh))
  (Variables|Default|SetStartPosition (Transformation|GetWorldLocation _mesh))
  (Variables|Default|SetStartRotation (Transformation|GetWorldRotation _mesh))
  (Variables|/Script/Engine.ProjectileMovementComponent|SetbSimulationEnabled (Variables|Default|GetProjectileMovement) false))

(event Collision|EventActorBeginOverlap
  (params (OtherActor :type Actor%20Object%20Reference)))

(event EventTick
  (params (DeltaSeconds :type Float%20%28single-precision%29)))

(fn ConstructionScript)